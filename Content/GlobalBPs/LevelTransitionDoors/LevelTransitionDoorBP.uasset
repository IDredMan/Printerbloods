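; Level transition door actor that teleports the first-person player to a linked SisterDoor.
; On a sending door, overlapping the Box plays a timeline that slides the door shut.
; After a short delay it moves the player to the sister's TPPoint, matches control rotation to that door and calls its OpenDoor, which reverses that door's timeline.
; The construction script starts non-sending doors closed.
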(event `self.Box.OnComponentBeginOverlap`
  (params (OverlappedComponent :type "PrimitiveComponent Object Reference") (OtherActor :type "Actor Object Reference") (OtherComp :type "PrimitiveComponent Object Reference") (OtherBodyIndex :type Integer) (bFromSweep :type Boolean) (SweepResult :type "HitResult Structure (by ref)"))
  (if (`self.SendingPlayer`)
    (bind _asbp_first_person_character (cast `/Game/FirstPerson/Blueprints/BP_FirstPersonCharacter` OtherActor))
    (set `self.FirstPersonCharacter` _asbp_first_person_character)
    (`|ExecutionSequence`
      (:`then_0`
        (bind (_direction _doorloclerp) (`Timeline|DoorCloseOpenTimeline` :!via `PlayFromStart`)
          (:`Update`
            (`SceneComponent.K2_SetRelativeLocation` (`self.Door`) (`KismetMathLibrary.MakeVector` 200.0 0.0 (`KismetMathLibrary.Lerp` 725.0 245.0 _doorloclerp)) false false))))
      (:`then_1`
        (`KismetSystemLibrary.Delay` 2.0)
        (`self.K2_SetActorLocation` (`self.FirstPersonCharacter`) (`SceneComponent.K2_GetComponentLocation` (`/Game/GlobalBPs/LevelTransitionDoors/LevelTransitionDoorBP.TPPoint` (`self.SisterDoor`))) false false)
        (`Controller.SetControlRotation` (`Pawn.GetController` (`self.FirstPersonCharacter`)) (`self.K2_GetActorRotation` (`self.SisterDoor`)))
        (`self.Open Door` (`self.SisterDoor`))))))

(event `Open Door`
  (`TimelineComponent.ReverseFromEnd` (`self.DoorCloseOpenTimeline`)))

(fn `UserConstructionScript`
  (if (not (`self.SendingPlayer`))
    (`SceneComponent.K2_SetRelativeLocation` (`self.Door`) (200.0 0.0 245.0) false false)))